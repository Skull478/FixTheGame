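; DMG_Zone is a damage zone that drains the health of a BP_CustomTPS character while it stands inside the Box component.
; Box begin and end overlap events set and clear a single Inside flag for that character class.
; While the flag is set, a looping Delay lowers Health and raises NNHealth0 by a fixed step every tenth of a second, with no limit check.
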(event `self.ReceiveActorBeginOverlap`
  (params (OtherActor :type "Actor Object Reference")))

(event `self.Box.OnComponentBeginOverlap`
  (params (OverlappedComponent :type "PrimitiveComponent Object Reference") (OtherActor :type "Actor Object Reference") (OtherComp :type "PrimitiveComponent Object Reference") (OtherBodyIndex :type Integer) (bFromSweep :type Boolean) (SweepResult :type "HitResult Structure (by ref)"))
  (bind _asbp_custom_tps (cast `/Game/Blueprints/Exportplugin/BP_CustomTPS` OtherActor))
  (bind _output_get (set `self.inside ?` true))
  (if _output_get :!label _label
    (set `/Game/Blueprints/Exportplugin/BP_CustomTPS.Health` (- (`/Game/Blueprints/Exportplugin/BP_CustomTPS.Health` _asbp_custom_tps) 1.0) _asbp_custom_tps)
    (set `/Game/Blueprints/Exportplugin/BP_CustomTPS.NN*Health_0` (+ (`/Game/Blueprints/Exportplugin/BP_CustomTPS.NN*Health_0` _asbp_custom_tps) 1.0) _asbp_custom_tps)
    (`KismetSystemLibrary.Delay` 0.1)
    (goto _label)))

(event `self.Box.OnComponentEndOverlap`
  (params (OverlappedComponent :type "PrimitiveComponent Object Reference") (OtherActor :type "Actor Object Reference") (OtherComp :type "PrimitiveComponent Object Reference") (OtherBodyIndex :type Integer))
  (cast `/Game/Blueprints/Exportplugin/BP_CustomTPS` OtherActor)
  (set `self.inside ?` false))

(fn `UserConstructionScript`)