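; Light stick pickup that the player collects with the interact input while standing inside its trigger sphere.
; Overlap with BP_CustomTPS shows Sphere1 and its children and starts a 0.2-second Delay loop polling the player's Interracting flag; leaving or another actor's overlap hides them.
; On interaction it spawns LightStickchara attached to the player mesh's RW socket, then destroys itself.
; Tick keeps the Widget turned toward the player's camera.
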(event `self.ReceiveBeginPlay`)

(event `self.ReceiveTick`
  (params (DeltaSeconds :type "Float (single-precision)"))
  (bind _widget (`self.Widget`))
  (bind _asbp_custom_tps (cast `/Game/Blueprints/Exportplugin/BP_CustomTPS` (`GameplayStatics.GetPlayerPawn` 0)))
  (`SceneComponent.K2_SetWorldRotation` _widget (`KismetMathLibrary.FindLookAtRotation` (`SceneComponent.K2_GetComponentLocation` _widget) (`SceneComponent.K2_GetComponentLocation` (`/Game/Blueprints/Exportplugin/BP_CustomTPS.Camera` _asbp_custom_tps))) false false))

(event `self.Sphere.OnComponentBeginOverlap`
  (params (OverlappedComponent :type "PrimitiveComponent Object Reference") (OtherActor :type "Actor Object Reference") (OtherComp :type "PrimitiveComponent Object Reference") (OtherBodyIndex :type Integer) (bFromSweep :type Boolean) (SweepResult :type "HitResult Structure (by ref)"))
  (bind _returnvalue (`GameplayStatics.GetPlayerCharacter` 0))
  (bind _sphere1 (`self.Sphere1`))
  (bind _mesh (`Character.Mesh` _returnvalue))
  (bind (_returnvalue_location _returnvalue_rotation _returnvalue_scale) (`KismetMathLibrary.BreakTransform` (`SceneComponent.GetSocketTransform` _mesh "RW" "RTS_World")))
  (cast `/Game/Blueprints/Exportplugin/BP_CustomTPS` OtherActor
    (:`then`
      (set `self.In` true)
      (`SceneComponent.SetVisibility` _sphere1 true true)
      (if (`self.In`) :!label _label
        (bind _asbp_custom_tps (cast `/Game/Blueprints/Exportplugin/BP_CustomTPS` _returnvalue))
        (if (`/Game/Blueprints/Exportplugin/BP_CustomTPS.Interracting ?` _asbp_custom_tps)
          (`/Engine/EditorBlueprintResources/StandardMacros.DoOnce` false
            (:`Completed`
              (bind _returnvalue_2 (`|SpawnActorFromClass` "/Game/Blueprints/Mécaniques/LightStickchara.LightStickchara_C" (`KismetMathLibrary.MakeTransform` _returnvalue_location _returnvalue_rotation _returnvalue_scale) "Undefined" "OverrideRootScale" null null))
              (`self.K2_AttachToComponent` _returnvalue_2 _mesh "RW" "SnapToTarget" "SnapToTarget" "SnapToTarget" true)
              (`self.K2_DestroyActor`)))
          (else
            (`KismetSystemLibrary.Delay` 0.2)
            (goto _label)))))
    (:`CastFailed`
      (set `self.In` false)
      (`SceneComponent.SetVisibility` _sphere1 false true :!label _label_2))))

(event `self.Sphere.OnComponentEndOverlap`
  (params (OverlappedComponent :type "PrimitiveComponent Object Reference") (OtherActor :type "Actor Object Reference") (OtherComp :type "PrimitiveComponent Object Reference") (OtherBodyIndex :type Integer))
  (cast `/Game/Blueprints/Exportplugin/BP_CustomTPS` OtherActor)
  (set `self.In` false)
  (goto _label_2))

(fn `UserConstructionScript`)